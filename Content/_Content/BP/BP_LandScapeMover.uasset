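; BP_LandScapeMover tracks the free-fall round timer, presumably to drive landscape movement, though no movement logic appears in this graph.
; On BeginPlay it caches BP_FreeFallGameMode, binds to its round start and end events, and calls Restart.
; Every Tick it polls the round's maximum time from the current parameters and the current time from the WBP_Timer UI widget, an approach the author flags as unoptimized.
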(event EventBeginPlay
  ;[1 1 1] Get timer and update it at each frame
  (bind _asbp_free_fall_game_mode (Utilities|Casting|CastToBP_FreeFallGameMode (Game|GetGameMode)))
  (EventDispatchers|BindEventtoOnStartRound _asbp_free_fall_game_mode (EventDispatchers|CreateEvent :!event Restart))
  (EventDispatchers|BindEventtoOnEndRound _asbp_free_fall_game_mode (EventDispatchers|CreateEvent :!event Pause))
  (Variables|Default|SetGameMode _asbp_free_fall_game_mode)
  (Class|LandscapeMoverActor|Restart))

(event EventTick
  (params (DeltaSeconds :type Float%20%28single-precision%29))
  ;[1 1 1] Get timer and update it at each frame
  ;;[1 1 1] Je sais c'est pas opti mais MERDE
  (bind _gamemode (Variables|Default|GetGameMode)
    (:then
      (bind _currentparameters (Variables|/Script/FreeFallingCouchGame.FreeFallGameMode|GetCurrentParameters _gamemode)
        (:then
          (Variables|Default|SetMaxTimer (Class|MatchParameters|GetRoundTimer _currentparameters))
          (bind _ingameui (Variables|/Game/_Content/BP/GameMode/BP_FreeFallGameMode.BP_FreeFallGameMode_C|GetInGameUI _gamemode)
            (:then
              (bind _aswbp_timer (Utilities|Casting|CastToWBP_Timer _ingameui))
              (Variables|Default|SetTimer (Variables|/Game/_Content/BP/UI/InGameUI/WBP_Timer.WBP_Timer_C|GetCurrentTime _aswbp_timer)))
            (:else)))
        (:else)))
    (:else)))

(fn ConstructionScript)