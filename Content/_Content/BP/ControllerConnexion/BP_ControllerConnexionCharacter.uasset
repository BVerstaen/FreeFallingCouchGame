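; Controller-connection screen character that stands in for one player slot and shows that player's chosen costume.
; Its skeletal mesh starts hidden and is revealed when LocalMultiplayerSubsystem creates the matching player (PlayerID minus one), which then unbinds and marks that player active in the game mode's map.
; Costume switch events from GameDataInstanceSubsystem look up the costume ID in DT_ListePersos and apply that row's material to the mesh.
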(event Custom|Switch%20Costume
  (params (IDCostume :type Integer) (IDplayer :type Integer))
  (|SwitchCostumeGraph IDCostume IDplayer))

(event Custom|ShowPlayer
  (params (NewPlayerID :type Integer))
  ;[1 1 1] Show player
  (if (== NewPlayerID (- (Variables|Default|GetPlayerID) 1))
    (bind _skeletalmesh (Variables|Default|GetSkeletalMesh)
      (:then
        (Development|SetHiddeninGame _skeletalmesh false false)
        (EventDispatchers|UnbindEventfromOnNewPlayerCreated (Subsystems|GetLocalMultiplayerSubsystem) (delegate Custom|ShowPlayer))
        (bind _asbp_controller_connexion_game_mode (Utilities|Casting|CastToBP_ControllerConnexionGameMode (Game|GetGameMode)))
        (Utilities|FlowControl|Delay 0.1)
        (Utilities|Map|Add (Variables|/Game/_Content/BP/GameMode/BP_ControllerConnexionGameMode.BP_ControllerConnexionGameMode_C|GetMapActivePlayers _asbp_controller_connexion_game_mode) (- (Variables|Default|GetPlayerID) 1) true))
      (:else))))

(event EventBeginPlay
  (EventDispatchers|BindEventtoOnCostumeSwitch (Subsystems|GetGameDataInstanceSubsystem) (delegate Custom|Switch%20Costume))
  (EventDispatchers|AssignOnNewPlayerCreated (Subsystems|GetLocalMultiplayerSubsystem) (delegate Custom|ShowPlayer))
  (bind _skeletalmesh (Variables|Default|GetSkeletalMesh)
    (:then
      (Development|SetHiddeninGame _skeletalmesh true false))
    (:else)))

(fn ConstructionScript)