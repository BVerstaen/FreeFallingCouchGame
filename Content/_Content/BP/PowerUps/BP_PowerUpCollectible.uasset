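; BP_PowerUpCollectible is a world pickup that gives a power-up to a FreeFallCharacter entering its sphere.
; On begin play it passes its power-up ID to an icon widget, which rotates toward the player camera every tick.
; Sphere overlaps call GivePowerToCharacter on entry and remove the character from the overlapping list on exit.
; A per-ID sphere material lookup is left unconnected, and a debug "Hello" print remains.
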(event OnComponentBeginOverlap(Sphere1)
  (params (OverlappedComponent :type Primitive%20Component%20Object%20Reference) (OtherActor :type Actor%20Object%20Reference) (OtherComp :type Primitive%20Component%20Object%20Reference) (OtherBodyIndex :type Integer) (bFromSweep :type Boolean) (SweepResult :type Hit%20Result%20Structure%20%28by%20ref%29))
  (bind _asfree_fall_character (Utilities|Casting|CastToFreeFallCharacter OtherActor))
  (Class|PowerUpCollectible|GivePowertoCharacter _asfree_fall_character))

(event OnComponentEndOverlap(Sphere1)
  (params (OverlappedComponent :type Primitive%20Component%20Object%20Reference) (OtherActor :type Actor%20Object%20Reference) (OtherComp :type Primitive%20Component%20Object%20Reference) (OtherBodyIndex :type Integer))
  (bind _asfree_fall_character (Utilities|Casting|CastToFreeFallCharacter OtherActor))
  (Class|PowerUpCollectible|RemoveCharacterfromOverlappingCharacters _asfree_fall_character))

(event EventBeginPlay
  (bind _returnvalue (Class|PowerUpCollectible|GetPowerUpID))
  (bind _aswbp_power_up_icon (Utilities|Casting|CastToWBP_PowerUpIcon (UserInterface|GetWidget (Variables|Default|GetWidget))))
  (Default|SetPowerUpIcon _aswbp_power_up_icon _returnvalue)
  (Development|PrintString "Hello"))

(event EventTick
  (params (DeltaSeconds :type Float%20%28single-precision%29))
  (bind _widget (Variables|Default|GetWidget))
  (Utilities|IsValid _widget
    (:Is%20Valid
      (Transformation|SetWorldRotation _widget (Math|Rotator|FindLookatRotation (Transformation|GetWorldLocation _widget) (Transformation|GetWorldLocation (Variables|/Script/Engine.PlayerCameraManager|GetTransformComponent (Game|GetPlayerCameraManager 0)))) false false))))

(fn ConstructionScript)