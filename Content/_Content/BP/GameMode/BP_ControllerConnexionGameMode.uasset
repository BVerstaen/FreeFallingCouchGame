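; Game mode for the controller connection menu, where local players join before the match starts.
; On BeginPlay it shows the connection widget, resets local players and costumes, opens the subsystem to new player creation and starts music.
; Each new-player callback increments a player count, and CE_StartGame opens the dive level only once at least two players have joined.
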(event Custom|CE_AddMaxNumberOfPlayer
  (params (NewPlayerID :type Integer))
  (Math|Integer|IncrementInt (Variables|Default|GetMaxNumberOfPlayers)))

(event Custom|CE_StartGame
  ;[1 1 1] Start Game
  (if (>= (Variables|Default|GetMaxNumberOfPlayers) 2)
    (Game|OpenLevel(byObjectReference) "/Game/_Content/Levels/GD/TestsAlexandreDiveLevels.TestsAlexandreDiveLevels")))

(event EventBeginPlay
  (bind _returnvalue (Subsystems|GetLocalMultiplayerSubsystem))
  (bind _returnvalue_2 (UserInterface|CreateWidget "/Game/_Content/BP/ControllerConnexion/WBP_ContollerConnexionMenu.WBP_ContollerConnexionMenu_C" (Game|GetPlayerController 0)))
  (UserInterface|Viewport|AddtoViewport _returnvalue_2 0)
  (Variables|/Game/_Content/BP/ControllerConnexion/WBP_ContollerConnexionMenu.WBP_ContollerConnexionMenu_C|SetGameMode _returnvalue_2 self)
  (Class|LocalMultiplayerSubsystem|ErasePlayers _returnvalue)
  (Class|LocalMultiplayerSubsystem|CreateandInitPlayers _returnvalue "Menu")
  (Class|LocalMultiplayerSubsystem|SetCanCreateNewPlayer _returnvalue true)
  (EventDispatchers|AssignOnNewPlayerCreated _returnvalue (delegate Custom|CE_AddMaxNumberOfPlayer))
  (Class|GameDataInstanceSubsystem|ResetPlayerCostumes (Subsystems|GetGameDataInstanceSubsystem))
  (Class|SoundSubsystem|PlayMusic (Subsystems|GetSoundSubsystem) (Variables|Default|GetMusic) 1.0 0.0))

(fn ConstructionScript)