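; Game mode for the main menu that sets up the menu screen, local multiplayer and video settings on BeginPlay.
; It creates the main menu widget, then resets the LocalMultiplayerSubsystem, initializes players for the menu and allows new players to be created.
; It also forces windowed mode at desktop resolution and scalability level 1 (Medium), although its inline comments say fullscreen and High.
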(event EventBeginPlay
  (bind _returnvalue (Subsystems|GetLocalMultiplayerSubsystem))
  (Utilities|FlowControl|Sequence
    (:then_0
      (bind _returnvalue_2 (UserInterface|CreateWidget "/Game/_Content/BP/UI/MainMenu/WBP_MainMenu.WBP_MainMenu_C" (Game|GetPlayerController 0)))
      (bind _output_get (Variables|Default|SetMainMenuRef _returnvalue_2))
      (UserInterface|Viewport|AddtoViewport _output_get 0)
      (Class|LocalMultiplayerSubsystem|ErasePlayers _returnvalue true)
      (Class|LocalMultiplayerSubsystem|CreateandInitPlayers _returnvalue "Menu")
      (Class|LocalMultiplayerSubsystem|SetCanCreateNewPlayer _returnvalue true))
    (:then_1
      ;[1 1 1] Set fullscreen & Desktop resolution
      (bind _returnvalue_3 (Settings|GetGameUserSettings))
      (Class|GameUserSettings|SetFullscreenMode _returnvalue_3 "Windowed")
      (Class|GameUserSettings|SetScreenResolution _returnvalue_3 (Class|GameUserSettings|GetDesktopResolution _returnvalue_3))
      (Class|GameUserSettings|ApplySettings _returnvalue_3 false)
      ;[1 1 1] Set graphics to High
      (Class|GameUserSettings|SetOverallScalabilityLevel _returnvalue_3 1)
      (Class|GameUserSettings|ApplySettings _returnvalue_3 false))))

(fn ConstructionScript)