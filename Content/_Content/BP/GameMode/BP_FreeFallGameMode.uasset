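; BP_FreeFallGameMode is the free-fall game mode Blueprint that manages in-game UI and pausing.
; BeginPlay creates a hidden in-game HUD, which ShowinGameUI later reveals and has find players.
; Only when CurrentRound is zero, it also adds a controls tutorial and hidden pause menu, starts looping wind ambience, and binds to round start.
; Round start binds player controllers' pause dispatchers to toggle the menu and game pause.
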(event Custom|CE_ScanPC
  ;[1 1 1] Create Pause Menu
  (bind _outactors (Actor|GetAllActorsOfClass "/Game/_Content/BP/Characters/BP_PC_GamePlayerController.BP_PC_GamePlayerController_C"))
  (for _array_element _outactors
    (EventDispatchers|BindEventtoEDonPause _array_element (delegate Custom|CE_TogglePause))))

(event Custom|CE_TogglePause
  ;[1 1 1] Create Pause Menu
  (bind _pauseui (Variables|Default|GetPauseUI)
    (:then
      (switch Utilities|FlowControl|Switch|SwitchonESlateVisibility (Variables|/Script/UMG.Widget|GetVisibility _pauseui)
        (:Visible
          (Widget|SetVisibility _pauseui "Hidden")
          (Game|SetGamePaused false))
        (:Hidden
          (Widget|SetVisibility _pauseui "Visible")
          (Game|SetGamePaused true))))
    (:else)))

(event EventShowinGameUI
  (bind _ingameui (Variables|Default|GetInGameUI))
  (Utilities|IsValid _ingameui
    (:Is%20Valid
      (Widget|SetVisibility _ingameui "Visible")
      (Default|FindPlayers _ingameui))))

(event EventBeginPlay
  ;[1 1 1] Create in game UI
  (bind _returnvalue (CallFunction|CreateWidget "Hidden" "/Game/_Content/BP/UI/InGameUI/WBP_InGameUI.WBP_InGameUI_C"))
  (bind _aswbp_in_game_ui (Utilities|Casting|CastToWBP_InGameUI _returnvalue))
  (Variables|Default|SetInGameUI _aswbp_in_game_ui)
  (if (== (Variables|/Script/FreeFallingCouchGame.GameDataInstanceSubsystem|GetCurrentRound (Subsystems|GetGameDataInstanceSubsystem)) 0)
    (bind _returnvalue_2 (CallFunction|CreateWidget "Visible" "/Game/_Content/BP/UI/InGameUI/WBP_ControlsTuto.WBP_ControlsTuto_C"))
    (bind _aswbp_controls_tuto (Utilities|Casting|CastToWBP_ControlsTuto _returnvalue_2))
    (Variables|Default|SetControlsTutoUI _aswbp_controls_tuto)
    ;[1 1 1] Create Pause Menu
    (bind _returnvalue_3 (CallFunction|CreateWidget "Hidden" "/Game/_Content/BP/UI/PauseMenu/WBP_MainPauseMenu.WBP_MainPauseMenu_C"))
    (bind _aswbp_main_pause_menu (Utilities|Casting|CastToWBP_MainPauseMenu _returnvalue_3))
    (Variables|Default|SetPauseUI _aswbp_main_pause_menu)
    (EventDispatchers|BindEventtoOnStartRound (delegate Custom|CE_ScanPC))
    (Class|SoundSubsystem|Play2DSound (Subsystems|GetSoundSubsystem) "AMB_3D_Wind_ST_Loop")))

(fn ConstructionScript)

(fn CreateWidget
  (params (InVisibility :type ESlateVisibility%20Enum :default "Visible") (Class :type User%20Widget%20Class%20Reference))
  (bind _returnvalue (UserInterface|CreateWidget Class))
  (Widget|SetVisibility _returnvalue InVisibility)
  (UserInterface|Viewport|AddtoViewport _returnvalue 0)
  (return _returnvalue))