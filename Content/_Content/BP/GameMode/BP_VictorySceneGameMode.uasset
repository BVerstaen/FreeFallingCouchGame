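; Game mode for the victory scene that sets up the end screen and its audio when play begins.
; It initializes local multiplayer players in Menu mode, blocks new player creation, shows the victory widget and starts victory ambience and music through the sound subsystem.
; An optional extra ambient sound also starts a looping timer, but its event is empty and the random PasList sound playback is disconnected.
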(event Custom|CE_Pas)

(event EventBeginPlay
  (bind _returnvalue (Subsystems|GetLocalMultiplayerSubsystem))
  (bind _returnvalue_2 (Subsystems|GetSoundSubsystem))
  (Class|LocalMultiplayerSubsystem|CreateandInitPlayers _returnvalue "Menu")
  (Class|LocalMultiplayerSubsystem|SetCanCreateNewPlayer _returnvalue false)
  (bind _returnvalue_3 (UserInterface|CreateWidget "/Game/_Content/BP/VictoryScreen/WBP_VictoryWidget.WBP_VictoryWidget_C" (Game|GetPlayerController 0)))
  (UserInterface|Viewport|AddtoViewport _returnvalue_3 0)
  (Class|SoundSubsystem|Play2DSound _returnvalue_2 (Variables|Default|GetVictoryAmb))
  (Class|SoundSubsystem|PlayMusic _returnvalue_2 "MUS_Victory_ST_Loop" 1.0 0.0)
  (bind _ambsound (Variables|Default|GetAmbSound)
    (:then
      (Audio|PlaySound2D _ambsound 1.0 1.0 0.0 0 0)
      (Utilities|Time|SetTimerbyEvent (delegate Custom|CE_Pas) (Variables|Default|GetPasDelay) true))
    (:else)))

(fn ConstructionScript)