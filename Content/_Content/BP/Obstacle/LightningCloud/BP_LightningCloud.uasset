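; Lightning cloud obstacle Blueprint that shows a cloud, a light beam and a triggered lightning strike effect.
; On BeginPlay it passes LightningRadius to two Niagara systems, scales the beam to match and deactivates the strike effect.
; When DirectionDependsOnCamera is set, beam and lightning rotate to LightningRotation with pitch offset 90 degrees.
; StruckLightning and TestLightning fire the strike effect, and PlaySound plays named 2D sounds from a map.
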(event Custom|Test%20Lightning
  (Components|Activation|Activate (Variables|Default|GetNiagara2) true))

(event EventBeginPlay
  (bind _lightningradius (Variables|Default|GetLightningRadius))
  (bind _lightningrotation (Variables|Default|GetLightningRotation))
  (bind _lightbeam (Variables|Default|GetLightBeam))
  (bind _lightningradius_2 (Variables|Default|GetLightningRadius))
  (bind _returnvalue (+ (.pitch _lightningrotation) 9e+01))
  (bind _returnvalue_2 (Math|Rotator|MakeRotator (.roll _lightningrotation) _returnvalue (.yaw _lightningrotation)))
  (Niagara|SetNiagaraVariable(Float) (Variables|Default|GetNiagara) "CloudRadius" _lightningradius_2)
  (Niagara|SetNiagaraVariable(Float) (Variables|Default|GetNiagara1) "CloudRadius" _lightningradius_2)
  (Components|Activation|Deactivate (Variables|Default|GetNiagara2))
  (Transformation|SetRelativeScale3D _lightbeam (Math|Vector|MakeVector (/ _lightningradius 14.0) (/ _lightningradius 14.0) 22.0))
  (if (Variables|Default|GetbDirectionDependsOnCamera)
    (Transformation|SetWorldRotation _lightbeam _returnvalue_2 false false)
    (Transformation|SetWorldRotation (Variables|Default|GetLightning) _returnvalue_2 false false)))

(event EventStruckLightning
  (Components|Activation|Activate (Variables|Default|GetNiagara2) true)
  (Development|PrintString "Hello"))

(event EventTick
  (params (DeltaSeconds :type Float%20%28single-precision%29)))

(event EventPlaySound
  (params (SoundName :type String))
  (bind _sounds (Variables|Default|GetSounds))
  (bind (_value _returnvalue) (Utilities|Map|Find _sounds SoundName))
  (if _returnvalue
    (Utilities|IsValid _value
      (:Is%20Valid
        (Audio|PlaySound2D _value 1.0 1.0 0.0 0 0)))))

(fn ConstructionScript)