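; BP_ObstacleVitrail is a stained-glass obstacle that shatters when the FreeFallCharacter hits it.
; On that hit it hides the static Mesh and shows the GeometryCollection in its place.
; It then spawns an FS_MasterField actor at the collection's location, sets its activation type and triggers it to drive the Chaos fracture.
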(event Collision|EventHit
  (params (MyComp :type Primitive%20Component%20Object%20Reference) (Other :type Actor%20Object%20Reference) (OtherComp :type Primitive%20Component%20Object%20Reference) (bSelfMoved :type Boolean) (HitLocation :type Vector :default "0, 0, 0") (HitNormal :type Vector :default "0, 0, 0") (NormalImpulse :type Vector :default "0, 0, 0") (Hit :type Hit%20Result%20Structure%20%28by%20ref%29))
  (Utilities|Casting|CastToFreeFallCharacter Other)
  (Rendering|SetVisibility (Variables|Default|GetGeometryCollection) true false)
  (Rendering|SetVisibility (Variables|Character|GetMesh) false false)
  (bind _returnvalue (Game|SpawnActorfromClass "/Engine/EditorResources/FieldNodes/FS_MasterField.FS_MasterField_C" (Math|Transform|MakeTransform (Transformation|GetWorldLocation (Variables|Default|GetGeometryCollection))) "Undefined" "MultiplyWithRoot" 0 0))
  (Variables|/Engine/EditorResources/FieldNodes/FS_MasterField.FS_MasterField_C|SetActivationType _returnvalue "NewEnumerator4")
  (Default|CETrigger _returnvalue))

(fn ConstructionScript)