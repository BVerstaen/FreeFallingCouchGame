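; BP_ObstacleSpawner is an obstacle spawner actor whose Blueprint graphs only provide debug visualization of its spawn area and obstacle direction.
; The construction script draws a short-lived green box at the actor's location and rotation, sized by ObstacleSpawnExtant.
; It also draws a line from the actor along ObstacleDirection, scaled by DebugDrawLineDistance.
; The event graph holds only disabled placeholder events, with no spawning logic.
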(event EventBeginPlay)

(event Collision|EventActorBeginOverlap
  (params (OtherActor :type Actor%20Object%20Reference)))

(event EventTick
  (params (DeltaSeconds :type Float%20%28single-precision%29)))

(fn ConstructionScript
  (Rendering|Debug|DrawDebugBox (Transformation|GetActorLocation) (Variables|Default|GetObstacleSpawnExtant) "(R=0.043133,G=1.000000,B=0.000000,A=1.000000)" (Transformation|GetActorRotation) 0.1 1.0)
  (Rendering|Debug|DrawDebugLine (Transformation|GetActorLocation) (+ (Transformation|GetActorLocation) (* (Variables|Default|GetObstacleDirection) (Variables|Default|GetDebugDrawLineDistance))) "(R=0.150092,G=1.000000,B=0.000000,A=1.000000)" 0.1 5.0))