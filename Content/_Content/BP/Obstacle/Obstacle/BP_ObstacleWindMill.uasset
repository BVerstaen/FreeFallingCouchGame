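; Windmill obstacle that toggles its mesh's physics constraint to lock and release position and rotation with its stable state.
; The constraint mode is None from BeginPlay, switches to Default on becoming stable, and returns to None when stability ends.
; Its bounce behaviour zeroes all linear and angular velocity, then resets the launch if it has never been stable, meaning it missed the correct height.
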(event EventBounceSpecificBehaviour
  (bind _mesh (Variables|Character|GetMesh)
    (:then
      (Class|PrimitiveComponent|SetAllPhysicsLinearVelocity _mesh "0, 0, 0" false)
      (Class|PrimitiveComponent|SetAllPhysicsAngularVelocityinDegrees _mesh (Math|Vector|MakeVectorNetQuantize 0.0 0.0 0.0) false)
      ;[1 1 1] Reset launch if didn't reach correct height
      (if (not (Variables|Default|GetbHasBeenStable))
        (Class|Obstacle|ResetLaunch)))
    (:else)))

(event EventEventBecommingStable
  ;[1 1 1] Lock & release position & rotation when is stable
  (bind _mesh (Variables|Character|GetMesh)
    (:then
      (Class|PrimitiveComponent|SetConstraintMode _mesh "Default"))
    (:else)))

(event EventBeginPlay
  ;[1 1 1] Lock & release position & rotation when is stable
  (bind _mesh (Variables|Character|GetMesh)
    (:then
      (Class|PrimitiveComponent|SetConstraintMode _mesh "None"))
    (:else)))

(event EventEventEndStable
  ;[1 1 1] Lock & release position & rotation when is stable
  (bind _mesh (Variables|Character|GetMesh)
    (:then
      (Class|PrimitiveComponent|SetConstraintMode _mesh "None"))
    (:else)))

(fn ConstructionScript)