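; BP_ObstacleLance is a lance obstacle that kills player characters in the free-fall game mode.
; When its mesh registers a hit, it runs a stationary box trace at its Box component, filtered to one object type, with persistent debug drawing.
; If the trace finds a BP_Character, it notifies BP_FreeFallGameMode of the death, then destroys the player with the Classic option.
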(event OnComponentHit(Mesh)
  (params (HitComponent :type Primitive%20Component%20Object%20Reference) (OtherActor :type Actor%20Object%20Reference) (OtherComp :type Primitive%20Component%20Object%20Reference) (NormalImpulse :type Vector :default "0, 0, 0") (Hit :type Hit%20Result%20Structure%20%28by%20ref%29))
  (bind _box (Variables|Default|GetBox))
  (bind _returnvalue (Transformation|GetWorldLocation _box))
  (bind (_outhit _returnvalue_2) (Class|KismetSystemLibrary|BoxTraceSingleforObjects _returnvalue _returnvalue (Components|Box|GetScaledBoxExtent _box) (Transformation|GetWorldRotation _box) (Utilities|Array|MakeArray "ObjectTypeQuery7") true 0 "Persistent" true))
  (if _returnvalue_2
    (bind _asbp_character (Utilities|Casting|CastToBP_Character (.HitActor (Collision|BreakHitResult _outhit))))
    (bind _asbp_free_fall_game_mode (Utilities|Casting|CastToBP_FreeFallGameMode (Game|GetGameMode)))
    (Class|FreeFallGameMode|CallArenaActoronCharacterDestroyed _asbp_free_fall_game_mode _asbp_character)
    (Class|FreeFallCharacter|DestroyPlayer _asbp_character "Classic")))

(event EventBeginPlay)

(event Collision|EventActorBeginOverlap
  (params (OtherActor :type Actor%20Object%20Reference)))

(event EventTick
  (params (DeltaSeconds :type Float%20%28single-precision%29)))

(fn ConstructionScript)