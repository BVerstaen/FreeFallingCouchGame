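; BP_TransitionClouds is a Niagara cloud effect that activates when a transition starts and deactivates when it completes.
; The construction script draws a brief debug box of the spawn extent, feeds particle and cloud size to Niagara, and uses ShowCloud for visibility and auto-activation.
; BeginPlay deactivates the effect, forces it visible, offsets it upward and passes in the end-transition delay.
; The transition events also print debug strings.
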(event EventOnTransitionStarted
  (Components|Activation|Activate (Variables|Default|GetNiagara) false)
  (Development|PrintString "Activate"))

(event EventOnTransitionCompleted
  (Components|Activation|Deactivate (Variables|Default|GetNiagara))
  (Development|PrintString "Deactivate"))

(event EventBeginPlay
  (bind _niagara (Variables|Default|GetNiagara))
  (Components|Activation|Deactivate _niagara)
  (Rendering|SetVisibility _niagara true false)
  (Transformation|SetRelativeLocation _niagara "0.000000,0.000000,60.000000" false false)
  (Effects|Components|ParticleSystem|SetFloatParameter _niagara "EndTransitionTime" (Variables|Default|GetDelayBeforeEndTransition)))

(fn ConstructionScript
  (bind _spawnextent (Variables|Default|GetSpawnExtent))
  (bind _niagara (Variables|Default|GetNiagara))
  (bind _showcloud (Variables|Default|GetShowCloud))
  (Rendering|Debug|DrawDebugBox (Transformation|GetActorLocation) _spawnextent "(R=0.000000,G=0.661372,B=1.000000,A=1.000000)" (Transformation|GetActorRotation) 0.3 1.0)
  (Niagara|SetNiagaraVariable(Float) _niagara "ParticleSize" (Variables|Default|GetParticleSize))
  (Niagara|SetNiagaraVariable(Vector3) _niagara "CloudSize" (* _spawnextent 2.0))
  (Rendering|SetVisibility _niagara _showcloud false)
  (Components|Activation|SetAutoActivate _niagara _showcloud))