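; BP_CameraMover drifts the main camera to random points around its start location and interrupts this for a timed camera event.
; BeginPlay attaches the camera, MoveWithCamActor and tagged actors to itself or that actor, separating move-only from move-and-rotate followers.
; StartCameraMovements begins a randomly delayed MoveComponentTo loop at CameraSpeed.
; TriggerEvent stops it, detaches MoveWithCamActor, moves out and back, then resumes, though GetEventCamLocationAndZRotation's target calculation is unconnected.
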(event Custom|MoveCamera
  (if (not (Variables|Event|GetisOnEvent))
    (bind (_targetrelativeposition _timetoreach) (CallFunction|FindNewPosition))
    (Components|MoveComponentTo (Variables|Default|GetDefaultSceneRoot) _targetrelativeposition "0, 0, 0" false false _timetoreach false)
    (if (not (Variables|Event|GetisOnEvent))
      (Utilities|FlowControl|Delay (Math|Random|RandomFloatinRange (Variables|Default|GetMinTimeBetweenMovements) (Variables|Default|GetMaxTimeBetweenMovements)))
      (if (not (Variables|Event|GetisOnEvent))
        (CallFunction|MoveCamera)))))

(event EventStartCameraMovements
  (Utilities|FlowControl|Delay (Variables|Default|GetStartingDelay))
  (CallFunction|MoveCamera))

(event EventTriggerEvent
  (bind (_location _zrotation) (|GetEventCamLocationandZRotation))
  (bind _eventmovementduration (Variables|Event|GetEventMovementDuration))
  (Development|PrintString "AHHHHHH")
  (Variables|Event|SetisOnEvent true)
  (Utilities|FlowControl|Sequence
    (:then_0
      (Components|MoveComponentTo (Variables|Default|GetDefaultSceneRoot) (stale Custom|MoveCamera _targetrelativeposition) "0, 0, 0" false false (stale Custom|MoveCamera _timetoreach) false) ; enters at Stop
    )
    (:then_1
      (Transformation|DetachFromActor (Variables|Components|GetMoveWithCamActor) "KeepWorld" "KeepWorld" "KeepWorld"))
    (:then_2
      (Variables|Event|SetBeforeEventLocation (Variables|/Script/Engine.SceneComponent|GetRelativeLocation (Variables|Default|GetDefaultSceneRoot)))
      (Development|PrintString (Utilities|String|ToString(Vector) _location) true true "(R=0.000000,G=0.660000,B=1.000000,A=1.000000)" 1e+02)
      (Components|MoveComponentTo (Variables|Default|GetDefaultSceneRoot) _location (Math|Rotator|MakeRotator 0.0 _zrotation 0.0) false false _eventmovementduration false)
      (Utilities|FlowControl|Delay (Variables|Event|GetEventDuration))
      (Components|MoveComponentTo (Variables|Default|GetDefaultSceneRoot) (Variables|Event|GetBeforeEventLocation) "0, 0, 0" false false _eventmovementduration false)
      (Class|CameraMoverActor|CallonEventEnded)
      (Variables|Event|SetisOnEvent false)
      (Transformation|AttachActorToActor (Variables|Components|GetMoveWithCamActor) self "None" "KeepWorld" "KeepWorld" "KeepWorld" true)
      (Utilities|FlowControl|Delay (Math|Random|RandomFloatinRange (Variables|Default|GetMinTimeBetweenMovements) (Variables|Default|GetMaxTimeBetweenMovements)))
      (CallFunction|MoveCamera))))

(event EventTick
  (params (DeltaSeconds :type Float%20%28single-precision%29))
  (Development|PrintString (Utilities|String|ToString(Vector) (Transformation|GetActorLocation (Variables|Default|GetMainCamera))) true true "(R=1.000000,G=0.319556,B=0.359370,A=1.000000)" DeltaSeconds))

(event EventBeginPlay
  (bind _self self)
  (bind _output_get (Variables|Default|SetBaseLocation (Transformation|GetActorLocation (Variables|Default|GetMainCamera))))
  (Utilities|IsValid (Variables|Components|GetMoveWithCamActor)
    (:Is%20Valid
      (Transformation|SetActorTransform (Math|Transform|MakeTransform _output_get "0, 0, 0" "1.000000,1.000000,1.000000"))
      (Transformation|AttachActorToActor (Variables|Default|GetMainCamera) _self "None" "KeepWorld" "KeepWorld" "KeepWorld" true)
      (Transformation|AttachActorToActor (Variables|Components|GetMoveWithCamActor) _self "None" "SnapToTarget" "SnapToTarget" "SnapToTarget" true)
      (bind _outactors (Actor|GetAllActorswithTag "MoveWithCamera"))
      (for _array_element _outactors
        (Transformation|AttachActorToActor _array_element (Variables|Components|GetMoveWithCamActor) "None" "KeepWorld" "KeepWorld" "KeepWorld" true))
      (Transformation|AttachActorToActor (Variables|Event|GetEventCameraTarget) (Variables|Components|GetMoveWithCamActor) "None" "KeepWorld" "KeepWorld" "KeepWorld" true)
      (bind _outactors_2 (Actor|GetAllActorswithTag "MoveAndRotateWithCamera"))
      (for _array_element_2 _outactors_2
        (Transformation|AttachActorToActor _array_element_2 self "None" "KeepWorld" "KeepWorld" "KeepWorld" true)))
    (:Is%20Not%20Valid
      (Development|PrintString "MoveWithCam Actor NOT SET" true true "(R=1.000000,G=0.000000,B=0.112128,A=1.000000)" 1e+03))))

(fn ConstructionScript)

(fn FindNewPosition
  (bind _array (Utilities|Array|MakeArray -1.0 1.0))
  (bind _maxdistance (Variables|Default|GetMaxDistance))
  (bind _mindistance (Variables|Default|GetMinDistance))
  (bind _output_get (LocalVariables|SetNew%20Position (+ (Variables|Default|GetBaseLocation) (Math|Vector|MakeVector (* (Math|Random|RandomFloatinRange _mindistance _maxdistance) (.OutItem (Utilities|Array|Random _array))) (* (Math|Random|RandomFloatinRange _mindistance _maxdistance) (.OutItem (Utilities|Array|Random _array))) 0.0))))
  (return _output_get (/ (Math|Vector|Distance(Vector) _output_get (Variables|Default|GetBaseLocation)) (Variables|Default|GetCameraSpeed))))

(fn SubtractTwoRotatorsBecauseUnrealCant
  (params (Rotator1 :type Rotator) (Rotator2 :type Rotator))
  (return (Math|Rotator|MakeRotator (- (.roll Rotator1) (.roll Rotator2)) (- (.pitch Rotator1) (.pitch Rotator2)) (- (.yaw Rotator1) (.yaw Rotator2)))))