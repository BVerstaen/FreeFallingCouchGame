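; BP_PC_Menu is a menu player controller in the VictoryScreen folder that turns Enhanced Input menu actions into event dispatcher broadcasts.
; Horizontal, vertical, accept and back each broadcast on press, with extra dispatchers for horizontal hold and accept release.
; It holds no menu logic itself, leaving the response to whatever binds to those dispatchers.
; A dead-zone and vertical-lock check remains in the graph but is disconnected.
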(event Input|EnhancedActionEvents|EnhancedInputActionIA_Menu_Vertical
  (params (ActionValue :type Float%20%28double-precision%29) (ElapsedSeconds :type Float%20%28double-precision%29) (TriggeredSeconds :type Float%20%28double-precision%29) (InputAction :type Input%20Action%20Object%20Reference :default "/Game/_Content/Input/Menu/IA_Menu_Vertical.IA_Menu_Vertical"))
  (:Started
    (Default|CallEDInputVertical ActionValue)))

(event Input|EnhancedActionEvents|EnhancedInputActionIA_Menu_Accept
  (params (ActionValue :type Boolean) (ElapsedSeconds :type Float%20%28double-precision%29) (TriggeredSeconds :type Float%20%28double-precision%29) (InputAction :type Input%20Action%20Object%20Reference :default "/Game/_Content/Input/Menu/IA_Menu_Accept.IA_Menu_Accept"))
  (:Started
    (Default|CallEDInputAccept))
  (:Completed
    (Default|CallEDInputAcceptReleased)))

(event Input|EnhancedActionEvents|EnhancedInputActionIA_Menu_Horizontal
  (params (ActionValue :type Float%20%28double-precision%29) (ElapsedSeconds :type Float%20%28double-precision%29) (TriggeredSeconds :type Float%20%28double-precision%29) (InputAction :type Input%20Action%20Object%20Reference :default "/Game/_Content/Input/Menu/IA_Menu_Horizontal.IA_Menu_Horizontal"))
  (:Triggered
    (if true
      (Default|CallEDInputHorizontalHold ActionValue)))
  (:Started
    (Default|CallEDInputHorizontal ActionValue)))

(event Input|EnhancedActionEvents|EnhancedInputActionIA_Menu_Back
  (params (ActionValue :type Boolean) (ElapsedSeconds :type Float%20%28double-precision%29) (TriggeredSeconds :type Float%20%28double-precision%29) (InputAction :type Input%20Action%20Object%20Reference :default "/Game/_Content/Input/Menu/IA_Menu_Back.IA_Menu_Back"))
  (:Started
    (Default|CallEDInputBack)))

(fn ConstructionScript)