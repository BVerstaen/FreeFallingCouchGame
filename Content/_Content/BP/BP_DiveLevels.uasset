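; BP_DiveLevels is a volume of three stacked dive layers that tracks the actors inside it implementing the DiveLayersSensible interface.
; The construction script sizes the top, middle and down boxes from DiveLevelSize, stacks them vertically and fits an enclosing collision box around them.
; A delayed BeginPlay scan and the begin-overlap event fill the tracked list without duplicates, printing debug text.
; End overlap does nothing, as its removal logic is disconnected.
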(event OnComponentBeginOverlap(DiveLayersCollisions)
  (params (OverlappedComponent :type Primitive%20Component%20Object%20Reference) (OtherActor :type Actor%20Object%20Reference) (OtherComp :type Primitive%20Component%20Object%20Reference) (OtherBodyIndex :type Integer) (bFromSweep :type Boolean) (SweepResult :type Hit%20Result%20Structure%20%28by%20ref%29))
  (bind _overlappingsensibleactors (Variables|Default|GetOverlappingSensibleActors))
  (if (Utilities|DoesObjectImplementInterface OtherActor "/Script/FreeFallingCouchGame.DiveLayersSensible")
    (bind _asdive_layers_sensible (Utilities|Casting|CastToDiveLayersSensible OtherActor))
    (if (not (Utilities|Array|ContainsItem _overlappingsensibleactors _asdive_layers_sensible))
      (Utilities|Array|Add _overlappingsensibleactors _asdive_layers_sensible)
      (Development|PrintString (Utilities|String|Append "Adding " (Utilities|GetDisplayName (stale OnComponentEndOverlap(DiveLayersCollisions) OtherActor))) true true "(R=1.000000,G=0.791072,B=0.000000,A=1.000000)"))))

(event OnComponentEndOverlap(DiveLayersCollisions)
  (params (OverlappedComponent :type Primitive%20Component%20Object%20Reference) (OtherActor :type Actor%20Object%20Reference) (OtherComp :type Primitive%20Component%20Object%20Reference) (OtherBodyIndex :type Integer)))

(event EventBeginPlay
  (bind _overlappingsensibleactors (Variables|Default|GetOverlappingSensibleActors))
  (Utilities|FlowControl|Delay 0.2)
  (for _array_element (Collision|GetOverlappingActors "/Script/Engine.Actor" :!class /Script/Engine.Actor)
    (if (Utilities|DoesObjectImplementInterface _array_element "/Script/FreeFallingCouchGame.DiveLayersSensible")
      (bind _asdive_layers_sensible (Utilities|Casting|CastToDiveLayersSensible _array_element))
      (if (not (Utilities|Array|ContainsItem _overlappingsensibleactors _asdive_layers_sensible))
        (Utilities|Array|Add _overlappingsensibleactors _asdive_layers_sensible)
        (Development|PrintString "Yep")))))

(fn ConstructionScript
  (bind _downlayer (Variables|Default|GetDownLayer))
  (bind _toplayer (Variables|Default|GetTopLayer))
  (bind _divelevelsize (Variables|Default|GetDiveLevelSize))
  (bind (_x _y _z) (Math|Vector|BreakVector _divelevelsize))
  (bind _returnvalue (* _z 2.0))
  (bind _returnvalue_2 (+ _returnvalue 1.0))
  (Components|Box|SetBoxExtent (Variables|Default|GetMiddleLayer) _divelevelsize true)
  (Components|Box|SetBoxExtent _toplayer _divelevelsize true)
  (Transformation|SetRelativeLocation _toplayer (Math|Vector|MakeVector 0.0 0.0 _returnvalue_2) false false)
  (Components|Box|SetBoxExtent _downlayer _divelevelsize true)
  (Transformation|SetRelativeLocation _downlayer (Math|Vector|MakeVector 0.0 0.0 (* _returnvalue_2 -1.0)) false false)
  (Components|Box|SetBoxExtent (Variables|Default|GetDiveLayersCollisions) (+ (Math|Vector|MakeVector _x _y (* _z 3.0)) "1.000000,1.000000,20.000000") true))