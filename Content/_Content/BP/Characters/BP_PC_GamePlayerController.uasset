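; Player controller Blueprint for the free-fall game that handles pause, menu and debug Enhanced Input actions.
; Pause and menu navigation, accept and back inputs are forwarded through CallED broadcast functions, with separate hold and release variants for horizontal and accept.
; Two invincibility actions cast to FreeFallGameMode and toggle camera death and player death.
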(event Input|EnhancedActionEvents|EnhancedInputActionIA_Pause
  (params (ActionValue :type Boolean) (ElapsedSeconds :type Float%20%28double-precision%29) (TriggeredSeconds :type Float%20%28double-precision%29) (InputAction :type Input%20Action%20Object%20Reference :default "/Game/_Content/Input/IA_Pause.IA_Pause"))
  (:Started
    (Default|CallEDonPause)))

(event Input|EnhancedActionEvents|EnhancedInputActionIA_InvincibleCamera
  (params (ActionValue :type Boolean) (ElapsedSeconds :type Float%20%28double-precision%29) (TriggeredSeconds :type Float%20%28double-precision%29) (InputAction :type Input%20Action%20Object%20Reference :default "/Game/_Content/Input/Debug/IA_InvincibleCamera.IA_InvincibleCamera"))
  (:Started
    (bind _asfree_fall_game_mode (Utilities|Casting|CastToFreeFallGameMode (Game|GetGameMode)))
    (Class|FreeFallGameMode|ToggleDisableCameraDeath _asfree_fall_game_mode)))

(event Input|EnhancedActionEvents|EnhancedInputActionIA_Menu_Vertical
  (params (ActionValue :type Float%20%28double-precision%29) (ElapsedSeconds :type Float%20%28double-precision%29) (TriggeredSeconds :type Float%20%28double-precision%29) (InputAction :type Input%20Action%20Object%20Reference :default "/Game/_Content/Input/Menu/IA_Menu_Vertical.IA_Menu_Vertical"))
  (:Started
    (Default|CallEDInputVertical ActionValue)))

(event Input|EnhancedActionEvents|EnhancedInputActionIA_Menu_Accept
  (params (ActionValue :type Boolean) (ElapsedSeconds :type Float%20%28double-precision%29) (TriggeredSeconds :type Float%20%28double-precision%29) (InputAction :type Input%20Action%20Object%20Reference :default "/Game/_Content/Input/Menu/IA_Menu_Accept.IA_Menu_Accept"))
  (:Started
    (Default|CallEDInputAccept))
  (:Completed
    (Default|CallEDInputAcceptReleased)))

(event Input|EnhancedActionEvents|EnhancedInputActionIA_Menu_Horizontal
  (params (ActionValue :type Float%20%28double-precision%29) (ElapsedSeconds :type Float%20%28double-precision%29) (TriggeredSeconds :type Float%20%28double-precision%29) (InputAction :type Input%20Action%20Object%20Reference :default "/Game/_Content/Input/Menu/IA_Menu_Horizontal.IA_Menu_Horizontal"))
  (:Triggered
    (Default|CallEDInputHorizontalHold ActionValue))
  (:Started
    (Default|CallEDInputHorizontal ActionValue)))

(event Input|EnhancedActionEvents|EnhancedInputActionIA_Menu_Back
  (params (ActionValue :type Boolean) (ElapsedSeconds :type Float%20%28double-precision%29) (TriggeredSeconds :type Float%20%28double-precision%29) (InputAction :type Input%20Action%20Object%20Reference :default "/Game/_Content/Input/Menu/IA_Menu_Back.IA_Menu_Back"))
  (:Started
    (Default|CallEDInputBack)))

(event Input|EnhancedActionEvents|EnhancedInputActionIA_InvinciblePlayer
  (params (ActionValue :type Boolean) (ElapsedSeconds :type Float%20%28double-precision%29) (TriggeredSeconds :type Float%20%28double-precision%29) (InputAction :type Input%20Action%20Object%20Reference :default "/Game/_Content/Input/Debug/IA_InvinciblePlayer.IA_InvinciblePlayer"))
  (:Started
    (bind _asfree_fall_game_mode (Utilities|Casting|CastToFreeFallGameMode (Game|GetGameMode)))
    (Class|FreeFallGameMode|ToggleDisablePlayerDeath _asfree_fall_game_mode)))

(fn ConstructionScript)