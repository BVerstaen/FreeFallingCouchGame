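; Player character Blueprint that handles world-space UI feedback over the player.
; On BeginPlay it shows a player-ID tag that timelines turn toward the camera, blink, then hide.
; De-grab events swap the tag for a blinking, camera-facing QTE widget, and power-up changes are forwarded through a call with the player index.
; Numpad keys force Idle or Move states for debugging; depth-material assignment is an empty stub, with dive-material code left unconnected.
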(event Custom|CE_PlayerTagAnimation
  ;[1 1 1] Blink player tag then hide him
  ;;[1 1 1] Set text
  (bind _playertagwidget (Variables|Default|GetPlayerTagWidget)
    (:then
      (bind _aswbp_player_tag (Utilities|Casting|CastToWBP_PlayerTag (UserInterface|GetWidget _playertagwidget)))
      (Default|CESetPlayerTagText _aswbp_player_tag (Class|FreeFallCharacter|GetIDPlayerLinked))
      (bind _playertagwidget_2 (Variables|Default|GetPlayerTagWidget)
        (:then
          (Rendering|SetVisibility _playertagwidget_2 true false)
          (Timeline|tl_PlayerTagLookAtCamera Play
            (:Update
              (bind _playertagwidget_3 (Variables|Default|GetPlayerTagWidget)
                (:then
                  (Transformation|SetWorldRotation _playertagwidget_3 (Math|Rotator|FindLookatRotation (Transformation|GetWorldLocation _playertagwidget_3) (Transformation|GetWorldLocation (Variables|/Script/Engine.PlayerCameraManager|GetTransformComponent (Game|GetPlayerCameraManager 0)))) false false))
                (:else)))
            (:Finished
              (bind _playertagwidget_4 (Variables|Default|GetPlayerTagWidget)
                (:then
                  (Rendering|SetVisibility _playertagwidget_4 false false))
                (:else)))
            (:Blink
              (bind _playertagwidget_5 (Variables|Default|GetPlayerTagWidget)
                (:then
                  (Rendering|ToggleVisibility _playertagwidget_5 false))
                (:else)))))
        (:else)))
    (:else)))

(event Custom|CE_AssignDepthMaterial
  ;[1 1 1] Assign depth material
)

(event Custom|CE_StopPlayerTagAnimation
  ;[1 1 1] Blink player tag then hide him
  (Timeline|tl_PlayerTagLookAtCamera Stop
    (:Update
      (bind _playertagwidget (Variables|Default|GetPlayerTagWidget)
        (:then
          (Transformation|SetWorldRotation _playertagwidget (Math|Rotator|FindLookatRotation (Transformation|GetWorldLocation _playertagwidget) (Transformation|GetWorldLocation (Variables|/Script/Engine.PlayerCameraManager|GetTransformComponent (Game|GetPlayerCameraManager 0)))) false false))
        (:else)))
    (:Finished
      (bind _playertagwidget_2 (Variables|Default|GetPlayerTagWidget)
        (:then
          (Rendering|SetVisibility _playertagwidget_2 false false))
        (:else)))
    (:Blink
      (bind _playertagwidget_3 (Variables|Default|GetPlayerTagWidget)
        (:then
          (Rendering|ToggleVisibility _playertagwidget_3 false))
        (:else)))))

(event EventActivateEffectDeGrab
  ;[1 1 1] DeGrab effect
  (CallFunction|CEStopPlayerTagAnimation)
  (bind _playertagwidget (Variables|Default|GetPlayerTagWidget)
    (:then
      (Rendering|SetVisibility _playertagwidget false false)
      (bind _degrabqtewidget (Variables|Default|GetDeGrabQTEWidget)
        (:then
          (Rendering|SetVisibility _degrabqtewidget true false)
          (Timeline|tl_DegrabQTELookAtCamera Play
            (:Update
              (bind _degrabqtewidget_2 (Variables|Default|GetDeGrabQTEWidget)
                (:then
                  (Transformation|SetWorldRotation _degrabqtewidget_2 (Math|Rotator|FindLookatRotation (Transformation|GetWorldLocation _degrabqtewidget_2) (Transformation|GetWorldLocation (Variables|/Script/Engine.PlayerCameraManager|GetTransformComponent (Game|GetPlayerCameraManager 0)))) false false))
                (:else)))
            (:Blink
              (bind _degrabqtewidget_3 (Variables|Default|GetDeGrabQTEWidget)
                (:then
                  (Rendering|ToggleVisibility _degrabqtewidget_3 false))
                (:else)))))
        (:else)))
    (:else)))

(event EventStopEffectDeGrab
  ;[1 1 1] DeGrab effect
  (bind _degrabqtewidget (Variables|Default|GetDeGrabQTEWidget)
    (:then
      (Rendering|SetVisibility _degrabqtewidget false false)
      (Timeline|tl_DegrabQTELookAtCamera Stop
        (:Update
          (bind _degrabqtewidget_2 (Variables|Default|GetDeGrabQTEWidget)
            (:then
              (Transformation|SetWorldRotation _degrabqtewidget_2 (Math|Rotator|FindLookatRotation (Transformation|GetWorldLocation _degrabqtewidget_2) (Transformation|GetWorldLocation (Variables|/Script/Engine.PlayerCameraManager|GetTransformComponent (Game|GetPlayerCameraManager 0)))) false false))
            (:else)))
        (:Blink
          (bind _degrabqtewidget_3 (Variables|Default|GetDeGrabQTEWidget)
            (:then
              (Rendering|ToggleVisibility _degrabqtewidget_3 false))
            (:else)))))
    (:else)))

(event EventUpdatePowerUpUI
  (params (PowerUpID :type EPowerUpsID%20Enum :default "None"))
  (Default|CallOnPowerUpChange (Class|FreeFallCharacter|GetIDPlayerLinked) PowerUpID))

(event EventBeginPlay
  (CallFunction|CEPlayerTagAnimation)
  (CallFunction|CEAssignDepthMaterial)
  ;[1 1 1] Hide DeGrab QTE Widget
  (bind _degrabqtewidget (Variables|Default|GetDeGrabQTEWidget)
    (:then
      (Rendering|ToggleVisibility _degrabqtewidget false))
    (:else)))

(event Input|KeyboardEvents|NumPadOne
  (params (Key :type Key%20Structure :default "None"))
  ;[1 1 1] Debug change state
  (:Pressed
    (Class|FreeFallCharacterStateMachine|ChangeState (Variables|Default|GetStateMachine) "Idle")))

(event Input|KeyboardEvents|NumPadTwo
  (params (Key :type Key%20Structure :default "None"))
  ;[1 1 1] Debug change state
  (:Pressed
    (Class|FreeFallCharacterStateMachine|ChangeState (Variables|Default|GetStateMachine) "Move")))

(fn ConstructionScript)