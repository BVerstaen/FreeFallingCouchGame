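; Player character for a free-fall game, handling its look, voice lines and overhead feedback.
; BeginPlay hides the widgets, binds the tag animation to the game mode, and scans a costume DataTable for material and voices, overwriting voices until the costume matches.
; Timelines turn the blinking player tag and de-grab QTE toward the camera and scale a crown on parachute pickup.
; Events also switch dive smoke, play voices and forward power-up UI changes.
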(event Custom|CE_PlayerTagAnimation
  ;[1 1 1] Blink player tag then hide him
  (bind _asbp_free_fall_game_mode (Utilities|Casting|CastToBP_FreeFallGameMode (Game|GetGameMode)))
  (EventDispatchers|UnbindEventfromEDonStartPlayerTagAnimation _asbp_free_fall_game_mode (EventDispatchers|CreateEvent :!event Custom|CE_PlayerTagAnimation))
  ;;[1 1 1] Set text
  (bind _playertagwidget (Variables|Default|GetPlayerTagWidget)
    (:then
      (bind _aswbp_player_tag (Utilities|Casting|CastToWBP_PlayerTag (UserInterface|GetWidget _playertagwidget)))
      (Default|CESetPlayerTagText _aswbp_player_tag (Class|FreeFallCharacter|GetIDPlayerLinked))
      (bind _playertagwidget_2 (Variables|Default|GetPlayerTagWidget)
        (:then
          (Rendering|SetVisibility _playertagwidget_2 true false)
          (Timeline|tl_PlayerTagLookAtCamera Play
            (:Update
              (bind _playertagwidget_3 (Variables|Default|GetPlayerTagWidget)
                (:then
                  (Transformation|SetWorldRotation _playertagwidget_3 (Math|Rotator|FindLookatRotation (Transformation|GetWorldLocation _playertagwidget_3) (Transformation|GetWorldLocation (Variables|/Script/Engine.PlayerCameraManager|GetTransformComponent (Game|GetPlayerCameraManager 0)))) false false))
                (:else)))
            (:Finished
              (bind _playertagwidget_4 (Variables|Default|GetPlayerTagWidget)
                (:then
                  (Rendering|SetVisibility _playertagwidget_4 false false))
                (:else)))
            (:Blink
              (bind _playertagwidget_5 (Variables|Default|GetPlayerTagWidget)
                (:then
                  (Rendering|ToggleVisibility _playertagwidget_5 false))
                (:else)))))
        (:else)))
    (:else)))

(event Custom|CE_AssignDepthMaterial
  ;[1 1 1] Assign depth material
)

(event Custom|CE_StopPlayerTagAnimation
  ;[1 1 1] Blink player tag then hide him
  (Timeline|tl_PlayerTagLookAtCamera Stop
    (:Update
      (bind _playertagwidget (Variables|Default|GetPlayerTagWidget)
        (:then
          (Transformation|SetWorldRotation _playertagwidget (Math|Rotator|FindLookatRotation (Transformation|GetWorldLocation _playertagwidget) (Transformation|GetWorldLocation (Variables|/Script/Engine.PlayerCameraManager|GetTransformComponent (Game|GetPlayerCameraManager 0)))) false false))
        (:else)))
    (:Finished
      (bind _playertagwidget_2 (Variables|Default|GetPlayerTagWidget)
        (:then
          (Rendering|SetVisibility _playertagwidget_2 false false))
        (:else)))
    (:Blink
      (bind _playertagwidget_3 (Variables|Default|GetPlayerTagWidget)
        (:then
          (Rendering|ToggleVisibility _playertagwidget_3 false))
        (:else)))))

(event Custom|CE_ShowCrownWidget
  ;[1 1 1] Parachute size evolution
  (CallFunction|CEStopPlayerTagAnimation)
  (bind _playertagwidget (Variables|Default|GetPlayerTagWidget)
    (:then
      (Rendering|SetVisibility _playertagwidget false false)
      (bind _crown (Variables|Default|GetCrown)
        (:then
          (Rendering|SetVisibility _crown true false)
          (bind _sizeevolution (Timeline|tl_CrownSizeAnimation Play)
            (:Update
              (bind _crown_2 (Variables|Default|GetCrown)
                (:then
                  (Transformation|SetRelativeScale3D _crown_2 (Math|Conversions|ToVector(Float) _sizeevolution)))
                (:else)))
            (:Finished
              (bind _crown_3 (Variables|Default|GetCrown)
                (:then
                  (Rendering|SetVisibility _crown_3 false false))
                (:else)))))
        (:else)))
    (:else)))

(event Custom|CE_HideCrownWidget
  ;[1 1 1] Parachute size evolution
  (bind _crown (Variables|Default|GetCrown)
    (:then
      (Rendering|SetVisibility _crown false false)
      (bind _sizeevolution (Timeline|tl_CrownSizeAnimation Stop)
        (:Update
          (bind _crown_2 (Variables|Default|GetCrown)
            (:then
              (Transformation|SetRelativeScale3D _crown_2 (Math|Conversions|ToVector(Float) _sizeevolution)))
            (:else)))
        (:Finished
          (bind _crown_3 (Variables|Default|GetCrown)
            (:then
              (Rendering|SetVisibility _crown_3 false false))
            (:else)))))
    (:else)))

(event EventActivateEffectDeGrab
  ;[1 1 1] DeGrab effect
  (CallFunction|CEStopPlayerTagAnimation)
  (bind _playertagwidget (Variables|Default|GetPlayerTagWidget)
    (:then
      (Rendering|SetVisibility _playertagwidget false false)
      (bind _degrabqtewidget (Variables|Default|GetDeGrabQTEWidget)
        (:then
          (Rendering|SetVisibility _degrabqtewidget true false)
          (Timeline|tl_DegrabQTELookAtCamera Play
            (:Update
              (bind _degrabqtewidget_2 (Variables|Default|GetDeGrabQTEWidget)
                (:then
                  (Transformation|SetWorldRotation _degrabqtewidget_2 (Math|Rotator|FindLookatRotation (Transformation|GetWorldLocation _degrabqtewidget_2) (Transformation|GetWorldLocation (Variables|/Script/Engine.PlayerCameraManager|GetTransformComponent (Game|GetPlayerCameraManager 0)))) false false))
                (:else)))
            (:Blink
              (bind _degrabqtewidget_3 (Variables|Default|GetDeGrabQTEWidget)
                (:then
                  (Rendering|ToggleVisibility _degrabqtewidget_3 false))
                (:else)))))
        (:else)))
    (:else)))

(event EventStopEffectDeGrab
  ;[1 1 1] DeGrab effect
  (bind _degrabqtewidget (Variables|Default|GetDeGrabQTEWidget)
    (:then
      (Rendering|SetVisibility _degrabqtewidget false false)
      (Timeline|tl_DegrabQTELookAtCamera Stop
        (:Update
          (bind _degrabqtewidget_2 (Variables|Default|GetDeGrabQTEWidget)
            (:then
              (Transformation|SetWorldRotation _degrabqtewidget_2 (Math|Rotator|FindLookatRotation (Transformation|GetWorldLocation _degrabqtewidget_2) (Transformation|GetWorldLocation (Variables|/Script/Engine.PlayerCameraManager|GetTransformComponent (Game|GetPlayerCameraManager 0)))) false false))
            (:else)))
        (:Blink
          (bind _degrabqtewidget_3 (Variables|Default|GetDeGrabQTEWidget)
            (:then
              (Rendering|ToggleVisibility _degrabqtewidget_3 false))
            (:else)))))
    (:else)))

(event EventUpdatePowerUpUI
  (params (PowerUpID :type EPowerUpsID%20Enum :default "None"))
  ;[1 1 1] Update Power Up UI
  (Default|CallOnPowerUpChange (Class|FreeFallCharacter|GetIDPlayerLinked) PowerUpID))

(event EventBeginPlay
  (bind _playertagwidget (Variables|Default|GetPlayerTagWidget)
    (:then
      (Rendering|SetVisibility _playertagwidget false false)
      (bind _asbp_free_fall_game_mode (Utilities|Casting|CastToBP_FreeFallGameMode (Game|GetGameMode)))
      (EventDispatchers|AssignEDonStartPlayerTagAnimation _asbp_free_fall_game_mode (EventDispatchers|CreateEvent :!event Custom|CE_PlayerTagAnimation))
      (CallFunction|CEAssignDepthMaterial)
      ;[1 1 1] Hide DeGrab QTE Widget
      (bind _degrabqtewidget (Variables|Default|GetDeGrabQTEWidget)
        (:then
          (Rendering|ToggleVisibility _degrabqtewidget false)
          ;[1 1 1] Hide Crown Widget
          (bind _crown (Variables|Default|GetCrown)
            (:then
              (Rendering|ToggleVisibility _crown false)
              ;[1 1 1] Set Texture
              (bind _returnvalue (Class|GameDataInstanceSubsystem|GetPlayerLookfromID (Subsystems|GetGameDataInstanceSubsystem) (Variables|Default|GetPlayerID)))
              (bind _outrownames (DataTable|GetDataTableRowNames "/Game/_Content/Data/DT_ListePersos.DT_ListePersos"))
              (bind _array_element (Utilities|Array|ForEachLoopwithBreak _outrownames :!label _label)
                (:LoopBody
                  (bind _returnvalue_2 (Utilities|GetDataTableRow "/Game/_Content/Data/DT_ListePersos.DT_ListePersos" _array_element)
                    (:then
                      (Utilities|Map|Add (Variables|Default|GetVoiceList) "Collision" (.collisionvoice _returnvalue_2))
                      (Utilities|Map|Add (Variables|Default|GetVoiceList) "GetPowerUp" (.getpowerupvoice _returnvalue_2))
                      (Utilities|Map|Add (Variables|Default|GetVoiceList) "Death" (.deathvoice _returnvalue_2))
                      (Utilities|Map|Add (Variables|Default|GetVoiceList) "Elimination" (.eliminationvoice _returnvalue_2))
                      (if (== (.id_costume _returnvalue_2) _returnvalue)
                        (bind _mesh (Variables|Character|GetMesh)
                          (:then
                            (Rendering|Material|SetMaterial _mesh 0 (.material _returnvalue_2))
                            (goto _label Break))
                          (:else))))))))
            (:else)))
        (:else)))
    (:else)))

(event EventOnParachuteGet
  (params (NewParachute :type Parachute%20Object%20Reference))
  ;[1 1 1] Parachute size evolution
  (CallFunction|CEShowCrownWidget))

(event EventOnParachuteLoss
  (params (PreviousParachute :type Parachute%20Object%20Reference))
  ;[1 1 1] Parachute size evolution
  (CallFunction|CEHideCrownWidget))

(event EventPlayVoiceSound
  (params (VoiceName :type String))
  (bind _voicelist (Variables|Default|GetVoiceList))
  (bind (_value _returnvalue) (Utilities|Map|Find _voicelist VoiceName))
  ;[1 1 1] Play voice sound
  (if _returnvalue
    (Utilities|IsValid _value
      (:Is%20Valid
        (Audio|PlaySoundatLocation _value (Transformation|GetActorLocation) "0, 0, 0" 1.0 1.0 0.0 0 0 0 0)))))

(event EventEnterDiveEvent
  (bind _smokeparticles (Variables|Default|GetSmokeParticles))
  ;[1 1 1] Dives
  (Class|NiagaraComponent|SetNiagaraVariableVec2 _smokeparticles "Velocity" (Variables|Niagara|GetVelocityParticlesDive))
  (Class|NiagaraComponent|SetNiagaraVariableVec2 _smokeparticles "Transparency" (Variables|Niagara|GetTransparencyParticlesHigh)))

(event EventExitDiveEvent
  (bind _smokeparticles (Variables|Default|GetSmokeParticles))
  ;[1 1 1] Dives
  (Class|NiagaraComponent|SetNiagaraVariableVec2 _smokeparticles "Velocity" (Variables|Niagara|GetVelocityParticlesBase))
  (Class|NiagaraComponent|SetNiagaraVariableVec2 _smokeparticles "Transparency" (Variables|Niagara|GetTransparencyParticlesLow)))

(event Input|KeyboardEvents|NumPadOne
  (params (Key :type Key%20Structure))
  ;[1 1 1] Debug change state
  (:Pressed
    (Class|FreeFallCharacterStateMachine|ChangeState (Variables|Default|GetStateMachine) "Idle")))

(event Input|KeyboardEvents|NumPadTwo
  (params (Key :type Key%20Structure))
  ;[1 1 1] Debug change state
  (:Pressed
    (Class|FreeFallCharacterStateMachine|ChangeState (Variables|Default|GetStateMachine) "Move")))

(fn ConstructionScript)