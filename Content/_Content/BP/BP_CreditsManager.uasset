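; Manager Blueprint for the credits, handling scene animations and the return to the main menu.
; ActivateAnimations plays each valid skeletal mesh component in the Animations array once without looping, printing a debug string for each.
; BeginPlay binds to the back input event on the BP_PC_Menu player controller.
; OnBackButtonPressed opens the L_MainMenu level.
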(event Custom|ActivateAnimations
  (for _array_element (Variables|Default|GetAnimations)
    (Utilities|IsValid (Variables|/Script/Engine.SkeletalMeshActor|GetSkeletalMeshComponent _array_element)
      (:Is%20Valid
        (Audio|Components|Audio|Play (Variables|/Script/Engine.SkeletalMeshActor|GetSkeletalMeshComponent _array_element) false)
        (Development|PrintString "Hello")))))

(event Custom|OnBackButtonPressed
  (Game|OpenLevel(byObjectReference) "/Game/_Content/Levels/L_MainMenu.L_MainMenu"))

(event EventBeginPlay
  (bind _asbp_pc_menu (Utilities|Casting|CastToBP_PC_Menu (Game|GetPlayerController 0)))
  (EventDispatchers|BindEventtoEDInputBack _asbp_pc_menu (EventDispatchers|CreateEvent :!event Custom|OnBackButtonPressed)))

(fn ConstructionScript)