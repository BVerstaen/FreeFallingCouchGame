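; BP_CameraHandler switches the player's view between scene cameras, looked up by camera state in the SceneCameras map.
; BeginPlay sets a default camera as view target.
; ChangeCameraState blends to the requested camera with optional shake, using a delay-cleared IsSwitching flag to block overlapping transitions and rejecting current or unmapped states.
; G, H and J keys trigger test transitions.
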(event Custom|ChangeCameraState
  (params (NewCamState :type E_CameraStates%20Enum :default "NewEnumerator4") (TransitionTime :type Float%20%28double-precision%29) (PlayCameraShake? :type Boolean))
  (bind _scenecameras (Variables|Default|GetSceneCameras))
  (bind (_value _returnvalue) (Utilities|Map|Find _scenecameras NewCamState))
  ;[1 1 1] Switch Camera
  (if (not (Utilities|Enum|Equal(Enum) NewCamState "NewEnumerator8"))
    (if (Variables|Default|GetIsSwitching) ; Checks if already switching
      (Development|PrintString "Wait for camera switching to end")
      (else
        (Development|PrintString "ChangeCamState")
        (if _returnvalue ; Checks if camera state is refered\nIn variable
          (if (== (Math|Conversions|ToInteger(Byte) NewCamState) (Math|Conversions|ToInteger(Byte) (Variables|Default|GetCurrentCamState))) ; Checks if we're in the passed state already
            (Development|PrintString "Already in this cam state")
            (else
              (Variables|Default|SetIsSwitching true)
              (Variables|Default|SetCurrentCamState NewCamState)
              (if PlayCameraShake? ; Checks if we need a camera shake\n (might replace with a function)
                (Game|Feedback|ClientStartCameraShake (Game|GetPlayerController 0) "/Game/_Content/BP/Camera/CameraShakes/BP_BaseCameraShake.BP_BaseCameraShake_C" 5e+01 "CameraLocal" "0, 0, 0"))
              (Game|Player|SetViewTargetwithBlend (Game|GetPlayerController 0) _value TransitionTime "VTBlend_Linear" 0.0 false)
              (Development|PrintString "Hello")
              (Utilities|FlowControl|Delay TransitionTime)
              (Variables|Default|SetIsSwitching false)))
          (else
            (Development|PrintString "That camera hasn't been setup,  look in the parameters of the BP_CameraHandler Instance you have in your scene !")))))))

(event EventBeginPlay
  (bind _scenecameras (Variables|Default|GetSceneCameras))
  (bind _value (Utilities|Map|Find _scenecameras "NewEnumerator7"))
  ;[1 1 1] Setup
  (Variables|Default|SetCurrent%20Camera _value)
  (Game|Player|SetViewTargetwithBlend (Game|GetPlayerController 0) _value 0.0 "VTBlend_Linear" 0.0 false))

(event Input|KeyboardEvents|J
  (params (Key :type Key%20Structure :default "None"))
  ;[1 0.2557 0.835] Test
  (:Pressed
    (CallFunction|ChangeCameraState "NewEnumerator1" 0.1 false)))

(event Input|KeyboardEvents|G
  (params (Key :type Key%20Structure :default "None"))
  ;[1 0.2557 0.835] Test
  (:Pressed
    (CallFunction|ChangeCameraState "NewEnumerator7" 3.0 false)))

(event Input|KeyboardEvents|H
  (params (Key :type Key%20Structure :default "None"))
  ;[1 0.2557 0.835] Test
  (:Pressed
    (CallFunction|ChangeCameraState "NewEnumerator0" 2.0 true)))

(fn ConstructionScript)