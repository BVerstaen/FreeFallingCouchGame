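; BP_Vitrail is a breakable stained-glass prop built on a Geometry Collection that reacts when a FreeFallCharacter hits it.
; The hit applies an impulse scaled from the character's velocity at the collection's world location, rather than at the contact point.
; It then spawns an FS_MasterField at that same location, sets its activation type and calls CETrigger on it.
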(event Collision|EventHit
  (params (MyComp :type Primitive%20Component%20Object%20Reference) (Other :type Actor%20Object%20Reference) (OtherComp :type Primitive%20Component%20Object%20Reference) (bSelfMoved :type Boolean) (HitLocation :type Vector :default "0, 0, 0") (HitNormal :type Vector :default "0, 0, 0") (NormalImpulse :type Vector :default "0, 0, 0") (Hit :type Hit%20Result%20Structure%20%28by%20ref%29))
  (bind _geometrycollection (Variables|Default|GetGeometryCollection))
  (bind _returnvalue (Transformation|GetWorldLocation _geometrycollection))
  (Utilities|Casting|CastToFreeFallCharacter Other)
  (Physics|AddImpulseatLocation (Variables|Default|GetGeometryCollection) (* (Transformation|GetVelocity Other) 1e+01) _returnvalue "None")
  (bind _returnvalue_2 (Game|SpawnActorfromClass "/Engine/EditorResources/FieldNodes/FS_MasterField.FS_MasterField_C" (Math|Transform|MakeTransform _returnvalue) "Undefined" "MultiplyWithRoot" 0 0))
  (Variables|/Engine/EditorResources/FieldNodes/FS_MasterField.FS_MasterField_C|SetActivationType _returnvalue_2 "NewEnumerator4")
  (Default|CETrigger _returnvalue_2))

(fn ConstructionScript)