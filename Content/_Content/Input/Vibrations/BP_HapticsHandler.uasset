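; BP_HapticsHandler triggers controller force feedback (rumble) for one player or all local players, apparently as a test setup.
; CallHapticsCollision prints debug text, then plays FFB_Test on the passed-in player controller if it is valid.
; CallHapticsAll loops over active platform users, resolves each one's player controller and plays a non-looping FFB_TestHeavy, without a validity check.
; An input-device controller lookup is left unconnected.
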(event EventCallHapticsCollision
  (params (Player :type Player%20Controller%20Object%20Reference))
  (Development|PrintText Player (Utilities|Text|FormatText "ID player is: {ID}" Player))
  (Development|PrintString Player "!!!!!!!!!!!!!!!!!!!!!!!!!!!!!!!!!!!!!!!!!!!!!!!!!!!!!!!!!!!!!!!!!!!!!!!!!!!!!!!!")
  (Utilities|IsValid Player
    (:Is%20Valid
      (Game|Feedback|ClientPlayForceFeedback Player "/Game/_Content/Input/Vibrations/FFB_Test.FFB_Test" "None" false false false))))

(event EventCallHapticsAll
  (bind _outusers (Class|InputDeviceLibrary|GetAllActiveUsers))
  (for _array_element _outusers
    (bind _returnvalue (Class|InputDeviceLibrary|GetPlayerControllerfromPlatformUser _array_element))
    (Game|Feedback|ClientPlayForceFeedback _returnvalue "/Game/_Content/Input/Vibrations/FFB_TestHeavy.FFB_TestHeavy" "None" false false false)))